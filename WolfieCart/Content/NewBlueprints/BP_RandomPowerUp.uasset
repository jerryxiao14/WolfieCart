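; BP_RandomPowerUp is a one-shot pickup for the car race that randomly applies an update or a decrement to the racer that touches it.
; Any sphere overlap prints a debug string and destroys the pickup before the racer type is checked.
; A cast chain identifies the player car or one of three NPCs, then a coin flip calls that racer's matching Update or Decrement function on BPCheckpoint.
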(event OnComponentBeginOverlap(Sphere)
  (params (OverlappedComponent :type Primitive%20Component%20Object%20Reference) (OtherActor :type Actor%20Object%20Reference) (OtherComp :type Primitive%20Component%20Object%20Reference) (OtherBodyIndex :type Integer) (bFromSweep :type Boolean) (SweepResult :type Hit%20Result%20Structure%20%28by%20ref%29))
  (bind _bp_checkpoint (Variables|Default|GetBP_Checkpoint))
  (bind _bp_checkpoint_2 (Variables|Default|GetBP_Checkpoint))
  (bind _bp_checkpoint_3 (Variables|Default|GetBP_Checkpoint))
  (bind _bp_checkpoint_4 (Variables|Default|GetBP_Checkpoint))
  (Development|PrintString "Random Powerup")
  (Actor|DestroyActor)
  (Utilities|Casting|CastToBP_PlayerCar OtherActor
    (:then
      (if (Math|Random|RandomBool)
        (Default|UpdatePlayer _bp_checkpoint_2 OtherActor)
        (else
          (Default|DecrementPlayer _bp_checkpoint_2 OtherActor))))
    (:CastFailed
      (Utilities|Casting|CastToBP_NPC1 OtherActor
        (:then
          (if (Math|Random|RandomBool)
            (Default|UpdateNPC1 _bp_checkpoint_3 OtherActor)
            (else
              (Default|DecrementNPC1 _bp_checkpoint_3 OtherActor))))
        (:CastFailed
          (Utilities|Casting|CastToBP_NPC2 OtherActor
            (:then
              (if (Math|Random|RandomBool)
                (Default|UpdateNPC2 _bp_checkpoint_4 OtherActor)
                (else
                  (Default|DecrementNpc2 _bp_checkpoint_4 OtherActor))))
            (:CastFailed
              (Utilities|Casting|CastToBP_NPC3 OtherActor)
              (if (Math|Random|RandomBool)
                (Default|UpdateNPC3 _bp_checkpoint OtherActor)
                (else
                  (Default|DecrementNpc3 _bp_checkpoint OtherActor))))))))))

(event EventBeginPlay)

(event Collision|EventActorBeginOverlap
  (params (OtherActor :type Actor%20Object%20Reference)))

(event EventTick
  (params (DeltaSeconds :type Float%20%28single-precision%29)))

(fn ConstructionScript)