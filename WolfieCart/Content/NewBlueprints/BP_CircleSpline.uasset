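; BP_CircleSpline is an actor Blueprint that shapes its spline component into an approximate circle at construction time.
; The construction script appends NumPoints points at Radius using sine and cosine, stepping by 350 divided by NumPoints degrees rather than 360.
; Points are placed in world space around the world origin at zero height, without clearing existing spline points.
; The event graph holds no active logic.
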(event EventBeginPlay)

(event Collision|EventActorBeginOverlap
  (params (OtherActor :type Actor%20Object%20Reference)))

(event EventTick
  (params (DeltaSeconds :type Float%20%28single-precision%29)))

(fn ConstructionScript
  (for _index (range 0 (- (Variables|Default|GetNumPoints) 1))
    (Spline|AddSplinePoint (Variables|Default|GetSpline) (Math|Vector|MakeVector (* (Variables|Default|GetRadius) (Math|Trig|Cos(Degrees) (Math|Conversions|ToFloat(Integer) (* (/ 350 (Variables|Default|GetNumPoints)) _index)))) (* (Math|Trig|Sin(Degrees) (Math|Conversions|ToFloat(Integer) (* (/ 350 (Variables|Default|GetNumPoints)) _index))) (Variables|Default|GetRadius)) 0.0) "World" true)))