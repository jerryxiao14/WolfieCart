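; Lap checkpoint for a car race that counts laps for the player and three NPC racers and decides the result.
; Box overlap casts the actor to player or NPC type, increments its lap count and writes it to BP_LapGameState.
; An NPC reaching LapsToWin is destroyed and clears PlayerCanWin, so the player later sees the lost widget instead of the win widget.
; Separate decrement events subtract a lap per racer.
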(event OnComponentBeginOverlap(Box)
  (params (OverlappedComponent :type Primitive%20Component%20Object%20Reference) (OtherActor :type Actor%20Object%20Reference) (OtherComp :type Primitive%20Component%20Object%20Reference) (OtherBodyIndex :type Integer) (bFromSweep :type Boolean) (SweepResult :type Hit%20Result%20Structure%20%28by%20ref%29))
  ;[0.15 0.15 0.15 0.5] Player Collides with Checkpoint
  ;;[0.15 0.15 0.15 0.5] Comment
  (bind _asbp_player_car (Utilities|Casting|CastToBP_PlayerCar OtherActor)
    (:then
      (CallFunction|UpdatePlayer _asbp_player_car))
    (:CastFailed
      ;;;[0.15 0.15 0.15 0.5] Comment
      (Utilities|Casting|CastToBP_NPC1 OtherActor
        (:then
          (CallFunction|UpdateNPC1 OtherActor))
        (:CastFailed
          (Utilities|Casting|CastToBP_NPC2 OtherActor
            (:then
              (CallFunction|UpdateNPC2 OtherActor))
            (:CastFailed
              (Utilities|Casting|CastToBP_NPC3 OtherActor)
              (CallFunction|UpdateNPC3 OtherActor))))))))

(event Custom|Display%20Win%20Menu
  ;[0.15 0.15 0.15 0.5] Display Win Menu
  (bind _returnvalue (UserInterface|CreateWidget "/Game/NewBlueprints/WBP_Won.WBP_Won_C"))
  (bind _output_get (Variables|Default|SetWonMenuRef _returnvalue))
  (UserInterface|Viewport|AddtoViewport _output_get 0))

(event Custom|Display%20Lost%20Menu
  ;[0.15 0.15 0.15 0.5] Display Lost Menu
  (bind _returnvalue (UserInterface|CreateWidget "/Game/NewBlueprints/WBP_Lost.WBP_Lost_C"))
  (bind _output_get (Variables|Default|SetLostMenuRef _returnvalue))
  (UserInterface|Viewport|AddtoViewport _output_get 0))

(event Custom|DecrementNpc3
  (params (Object :type Actor%20Object%20Reference))
  (bind _asbp_npc3 (Utilities|Casting|CastToBP_NPC3 Object))
  (bind _output_get (Variables|/Game/VehicleTemplate/Blueprints/SportsCar/BP_NPC3.BP_NPC3_C|SetLapsCompleted _asbp_npc3 (+ (Variables|/Game/VehicleTemplate/Blueprints/SportsCar/BP_NPC3.BP_NPC3_C|GetLapsCompleted _asbp_npc3) -1)))
  (Variables|/Game/NewBlueprints/BP_LapGameState.BP_LapGameState_C|SetNPC3Laps (Variables|Default|GetAs%20BP%20Lap%20Game%20State) _output_get))

(event Custom|Display%20Menu
  ;[0.15 0.15 0.15 0.5] Display Menu
  (if (Variables|Default|GetPlayerCanWin)
    (CallFunction|DisplayWinMenu)
    (else
      (CallFunction|DisplayLostMenu))))

(event Custom|Update%20Player
  (params (NewParam :type Actor%20Object%20Reference))
  ;[0.15 0.15 0.15 0.5] Update Player
  (bind _asbp_player_car (Utilities|Casting|CastToBP_PlayerCar NewParam))
  (Variables|Default|SetPlayerActor _asbp_player_car)
  (bind _result (Math|Integer|IncrementInt (Variables|/Game/VehicleTemplate/Blueprints/SportsCar/BP_PlayerCar.BP_PlayerCar_C|GetLapsCompleted _asbp_player_car))
    (:%20%20
      (bind _output_get (Variables|/Game/VehicleTemplate/Blueprints/SportsCar/BP_PlayerCar.BP_PlayerCar_C|SetLapsCompleted _asbp_player_car _result))
      (Variables|/Game/NewBlueprints/BP_LapGameState.BP_LapGameState_C|SetPlayerLaps (Variables|Default|GetAs%20BP%20Lap%20Game%20State) _output_get)
      (if (>= _output_get (Variables|Default|GetLapsToWin))
        (CallFunction|DisplayMenu)))))

(event Custom|Decrement%20Player
  (params (Player :type Actor%20Object%20Reference))
  (bind _asbp_player_car (Utilities|Casting|CastToBP_PlayerCar Player))
  (bind _output_get (Variables|/Game/VehicleTemplate/Blueprints/SportsCar/BP_PlayerCar.BP_PlayerCar_C|SetLapsCompleted _asbp_player_car (+ (Variables|/Game/VehicleTemplate/Blueprints/SportsCar/BP_PlayerCar.BP_PlayerCar_C|GetLapsCompleted _asbp_player_car) -1)))
  (Variables|/Game/NewBlueprints/BP_LapGameState.BP_LapGameState_C|SetPlayerLaps (Variables|Default|GetAs%20BP%20Lap%20Game%20State) _output_get))

(event Custom|DecrementNPC1
  (params (Object :type Actor%20Object%20Reference))
  (bind _asbp_npc1 (Utilities|Casting|CastToBP_NPC1 Object))
  (bind _output_get (Variables|/Game/VehicleTemplate/Blueprints/SportsCar/BP_NPC1.BP_NPC1_C|SetLapsCompleted _asbp_npc1 (+ (Variables|/Game/VehicleTemplate/Blueprints/SportsCar/BP_NPC1.BP_NPC1_C|GetLapsCompleted _asbp_npc1) -1)))
  (Variables|/Game/NewBlueprints/BP_LapGameState.BP_LapGameState_C|SetNPC1Laps (Variables|Default|GetAs%20BP%20Lap%20Game%20State) _output_get))

(event Custom|Update%20NPC1
  (params (Object%20Ref :type Actor%20Object%20Reference))
  ;[0.15 0.15 0.15 0.5] Update NPC1
  (bind _asbp_npc1 (Utilities|Casting|CastToBP_NPC1 Object%20Ref))
  (bind _result (Math|Integer|IncrementInt (Variables|/Game/VehicleTemplate/Blueprints/SportsCar/BP_NPC1.BP_NPC1_C|GetLapsCompleted _asbp_npc1))
    (:%20%20
      (bind _output_get (Variables|/Game/VehicleTemplate/Blueprints/SportsCar/BP_NPC1.BP_NPC1_C|SetLapsCompleted _asbp_npc1 _result))
      (Default|SetNPC1Score (Variables|Default|GetAs%20BP%20Lap%20Game%20State) _output_get)
      (if (>= _output_get (Variables|Default|GetLapsToWin))
        (Actor|DestroyActor Object%20Ref)
        (if (Variables|Default|GetPlayerCanWin)
          (Variables|Default|SetPlayerCanWin false))))))

(event Custom|Update%20NPC2
  (params (Object%20Ref :type Actor%20Object%20Reference))
  ;[0.15 0.15 0.15 0.5] Update NPC2
  (bind _asbp_npc2 (Utilities|Casting|CastToBP_NPC2 Object%20Ref))
  (bind _result (Math|Integer|IncrementInt (Variables|/Game/VehicleTemplate/Blueprints/SportsCar/BP_NPC2.BP_NPC2_C|GetLapsCompleted _asbp_npc2))
    (:%20%20
      (bind _output_get (Variables|/Game/VehicleTemplate/Blueprints/SportsCar/BP_NPC2.BP_NPC2_C|SetLapsCompleted _asbp_npc2 _result))
      (Default|SetNPC2Score (Variables|Default|GetAs%20BP%20Lap%20Game%20State) _output_get)
      (if (>= _output_get (Variables|Default|GetLapsToWin))
        (Actor|DestroyActor Object%20Ref)
        (if (Variables|Default|GetPlayerCanWin)
          (Variables|Default|SetPlayerCanWin false))))))

(event Custom|Update%20NPC3
  (params (Object%20Ref :type Actor%20Object%20Reference))
  ;[0.15 0.15 0.15 0.5] Update NPC3
  (bind _asbp_npc3 (Utilities|Casting|CastToBP_NPC3 Object%20Ref))
  (bind _result (Math|Integer|IncrementInt (Variables|/Game/VehicleTemplate/Blueprints/SportsCar/BP_NPC3.BP_NPC3_C|GetLapsCompleted _asbp_npc3))
    (:%20%20
      (bind _output_get (Variables|/Game/VehicleTemplate/Blueprints/SportsCar/BP_NPC3.BP_NPC3_C|SetLapsCompleted _asbp_npc3 _result))
      (Default|SetNPC3Score (Variables|Default|GetAs%20BP%20Lap%20Game%20State) _output_get)
      (if (>= _output_get (Variables|Default|GetLapsToWin))
        (Actor|DestroyActor Object%20Ref)
        (if (Variables|Default|GetPlayerCanWin)
          (Variables|Default|SetPlayerCanWin false))))))

(event Custom|DecrementNpc2
  (params (Object :type Actor%20Object%20Reference))
  (bind _asbp_npc2 (Utilities|Casting|CastToBP_NPC2 Object))
  (bind _output_get (Variables|/Game/VehicleTemplate/Blueprints/SportsCar/BP_NPC2.BP_NPC2_C|SetLapsCompleted _asbp_npc2 (+ (Variables|/Game/VehicleTemplate/Blueprints/SportsCar/BP_NPC2.BP_NPC2_C|GetLapsCompleted _asbp_npc2) -1)))
  (Variables|/Game/NewBlueprints/BP_LapGameState.BP_LapGameState_C|SetNPC2Laps (Variables|Default|GetAs%20BP%20Lap%20Game%20State) _output_get))

(event Collision|EventActorBeginOverlap
  (params (OtherActor :type Actor%20Object%20Reference)))

(event EventTick
  (params (DeltaSeconds :type Float%20%28single-precision%29)))

(event EventBeginPlay
  (Development|PrintString "Hello")
  (bind _asbp_lap_game_state (Utilities|Casting|CastToBP_LapGameState (Game|GetGameState)))
  (Variables|Default|SetAs%20BP%20Lap%20Game%20State _asbp_lap_game_state))

(fn ConstructionScript)