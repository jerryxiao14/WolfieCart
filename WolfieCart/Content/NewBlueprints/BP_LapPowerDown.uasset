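; BP_LapPowerDown is a racing pickup that triggers a decrement, apparently of laps, for the car that touches it.
; Any overlap with its Sphere destroys the actor first, even if the other actor is not a racer.
; A cast chain then identifies the player car or one of three NPC types and calls the matching Decrement function on BPCheckpoint.
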(event OnComponentBeginOverlap(Sphere)
  (params (OverlappedComponent :type Primitive%20Component%20Object%20Reference) (OtherActor :type Actor%20Object%20Reference) (OtherComp :type Primitive%20Component%20Object%20Reference) (OtherBodyIndex :type Integer) (bFromSweep :type Boolean) (SweepResult :type Hit%20Result%20Structure%20%28by%20ref%29))
  (Actor|DestroyActor)
  (Utilities|Casting|CastToBP_PlayerCar OtherActor
    (:then
      (Default|DecrementPlayer (Variables|Default|GetBP_Checkpoint) OtherActor))
    (:CastFailed
      (Utilities|Casting|CastToBP_NPC1 OtherActor
        (:then
          (Default|DecrementNPC1 (Variables|Default|GetBP_Checkpoint) OtherActor))
        (:CastFailed
          (Utilities|Casting|CastToBP_NPC2 OtherActor
            (:then
              (Default|DecrementNpc2 (Variables|Default|GetBP_Checkpoint) OtherActor))
            (:CastFailed
              (Utilities|Casting|CastToBP_NPC3 OtherActor)
              (Default|DecrementNpc3 (Variables|Default|GetBP_Checkpoint) OtherActor))))))))

(event EventBeginPlay)

(event Collision|EventActorBeginOverlap
  (params (OtherActor :type Actor%20Object%20Reference)))

(event EventTick
  (params (DeltaSeconds :type Float%20%28single-precision%29)))

(fn ConstructionScript)